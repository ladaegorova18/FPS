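; AI controller for AI_Base enemies that runs AI_MainTree and treats player character 0 as the enemy.
; On BeginPlay it stores the player in the AI_Blackboard "Enemy" key and caches the controlled pawn.
; Perception updates for the player write the first stimulus's sensed state to "CanSeePlayer".
; If the player is sensed while the pawn is crouching, it also clears "IsInCover".
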(event `self.ReceiveBeginPlay`
  (`self.RunBehaviorTree` "/Game/Blueprints/AI/AI_MainTree.AI_MainTree")
  (set `self.Enemy` (`GameplayStatics.GetPlayerCharacter` 0))
  (bind _blackboardcomponent (`self.UseBlackboard` "/Game/Blueprints/AI/AI_Blackboard.AI_Blackboard"))
  (`BlackboardComponent.SetValueAsObject` _blackboardcomponent "Enemy" (`self.Enemy`))
  (bind _asaichar (cast `/Game/Blueprints/AI_Base` (`self.K2_GetPawn`)))
  (set `self.EnemyPawn` _asaichar))

(event `self.AIPerception.OnPerceptionUpdated`
  (params (UpdatedActors :type "Array of Actor Object Reference (by ref)"))
  (for _array_element UpdatedActors
    (if (== _array_element (`self.Enemy`))
      (bind _info (`AIPerceptionComponent.GetActorsPerception` (`self.AIPerception`) _array_element))
      (bind _output_get (set `self.CanSeePlayer` (`.bSuccessfullySensed` (break `AIStimulus` (`|GetArrayItem` (`.LastSensedStimuli` (break `ActorPerceptionBlueprintInfo` _info)))))))
      (`BlackboardComponent.SetValueAsBool` (`AIBlueprintHelperLibrary.GetBlackboard` null) "CanSeePlayer" _output_get)
      (if (and (`self.CanSeePlayer`) (`NavMovementComponent.IsCrouching` (`Character.CharacterMovement` (`self.EnemyPawn`))))
        (`BlackboardComponent.SetValueAsBool` (`AIBlueprintHelperLibrary.GetBlackboard` null) "IsInCover" false)))))

(fn `UserConstructionScript`)