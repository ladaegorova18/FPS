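; Behavior tree task that makes an AI_Base enemy attack for as long as the task runs.
; On execute it starts the pawn's attack, then switches the controller to the EnemyShootCover tree if the blackboard cover location is within 1000 units and the pawn is not already in cover.
; It never calls Finish Execute, so it stays active until aborted, when it stops the attack.
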(event `self.ReceiveExecuteAI`
  (params (OwnerController :type "AIController Object Reference") (ControlledPawn :type "Pawn Object Reference"))
  ;[1 1 1] Start Attack
  (bind _output_get (set `self.Pawn` ControlledPawn))
  (bind _asai_base (cast `/Game/Blueprints/AI/AI_Base` _output_get))
  (`/Game/Blueprints/AI/AI_Base.StartAttack` _asai_base)
  (bind _iscoverclose (`self.IsCoverClose`))
  (if _iscoverclose
    (`AIController.RunBehaviorTree` OwnerController "/Game/Blueprints/AI/ShootAttack/EnemyShootCover.EnemyShootCover")))

(event `self.ReceiveAbortAI`
  (params (OwnerController :type "AIController Object Reference") (ControlledPawn :type "Pawn Object Reference"))
  ;[1 1 1] Stop Attack
  (bind _asai_base (cast `/Game/Blueprints/AI/AI_Base` ControlledPawn))
  (`/Game/Blueprints/AI/AI_Base.StopAttack` _asai_base)
  (`self.FinishAbort`))

(fn `IsCoverClose`
  (returns (IsCoverClose :type Boolean))
  (return (and (< (`KismetMathLibrary.Vector_Distance` (`BTFunctionLibrary.GetBlackboardValueAsVector` (`self.BB_CoverLocation`)) (`Actor.K2_GetActorLocation` (`self.Pawn`))) 1000.0) (not (`BTFunctionLibrary.GetBlackboardValueAsBool` (`self.BB_IsInCover`))))))