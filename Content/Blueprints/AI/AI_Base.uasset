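; Base AI enemy character with health, cover crouching and ranged or melee attacks, driven by behavior trees and blackboard values set at BeginPlay.
; A threat switches it to the shoot-from-cover tree facing the source, and leaving cover restores the main tree.
; Attacks use the socket-attached child-actor weapon or an empty StartMeleeAttack function.
; Damage plays a hit reaction or, at zero health, stops the AI, ragdolls and destroys it after a delay.
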(event `Threatened`
  (params (ThreatSource :type "Vector Structure"))
  (bind _returnvalue (`AIBlueprintHelperLibrary.GetAIController` self))
  ;[1 1 1] Get Damage
  (`AIController.RunBehaviorTree` _returnvalue "/Game/Blueprints/AI/ShootAttack/EnemyShootCover.EnemyShootCover")
  (`AIController.K2_SetFocalPoint` _returnvalue ThreatSource))

(event `CheckHealth`
  ;[1 1 1] Check health level and die
  (if (<= (`self.Health`) 0.0)
    (`PrimitiveComponent.SetSimulatePhysics` (`self.Mesh`) true)
    (`BrainComponent.StopLogic` (`AIController.BrainComponent` (`AIBlueprintHelperLibrary.GetAIController` self)) "")
    (`PrimitiveComponent.SetCollisionEnabled` (`self.CapsuleComponent`) "NoCollision")
    (`PrimitiveComponent.SetCollisionResponseToChannel` (`self.Mesh`) "ECC_Pawn" "ECR_Ignore")
    (`self.StopAttack`)
    (`KismetSystemLibrary.Delay` 20.0)
    (`self.K2_DestroyActor`)
    (else
      (`|PlayMontage` (`self.Mesh`) "/Game/AnimStarterPack/React_Montage.React_Montage"))))

(event `self.ReceiveAnyDamage`
  (params (Damage :type "Float (single-precision)") (DamageType :type "DamageType Object Reference") (InstigatedBy :type "Controller Object Reference") (DamageCauser :type "Actor Object Reference"))
  ;[1 1 1] Get Damage
  (set `self.Health` (- (`self.Health`) Damage))
  (`self.CheckHealth`))

(event `StartAttack`
  ;[1 1 1] Start/Stop Shooting
  (if (`|EnumEquality` (`self.AttackType`) "NewEnumerator1")
    (`/Game/Assets/Guns/Weapon.StartShooting` (`self.CurrentGun`))
    (else
      (`self.StartMeleeAttack`))))

(event `GetOutOfCover`
  ;[1 1 1] Enter/Get out of cover
  (set `self.IsInCover` false)
  (`self.UnCrouch`)
  (bind _asaicontrol (cast `/Game/Blueprints/AI/AIControl` (`AIBlueprintHelperLibrary.GetAIController` self)))
  (`AIController.RunBehaviorTree` _asaicontrol "/Game/Blueprints/AI/AI_MainTree.AI_MainTree"))

(event `StopAttack`
  ;[1 1 1] Start/Stop Shooting
  (if (`|EnumEquality` (`self.AttackType`) "NewEnumerator1")
    (`/Game/Assets/Guns/Weapon.StopShooting` (`self.CurrentGun`))))

(event `EnterCover`
  ;[1 1 1] Enter/Get out of cover
  (set `self.IsInCover` true)
  (`self.Crouch`)
  (cast `/Game/Blueprints/AI/AIControl` (`AIBlueprintHelperLibrary.GetAIController` self)))

(event `Play Shoot FX`
  (bind _gun (`self.Gun`))
  (`GameplayStatics.SpawnEmitterAtLocation` null (`SceneComponent.GetSocketLocation` _gun "Socket") (`SceneComponent.GetSocketRotation` _gun "Socket")))

(event `self.ReceiveBeginPlay`
  (bind _returnvalue (`AIBlueprintHelperLibrary.GetBlackboard` null))
  ;[1 1 1] Set Blackboard values
  (`BlackboardComponent.SetValueAsEnum` _returnvalue "AttackType" (`self.AttackType`))
  (`BlackboardComponent.SetValueAsBool` _returnvalue "Static" (`self.Static`)))

(fn `StartMeleeAttack`)

(fn `UserConstructionScript`
  ;[1 1 1] Attach weapon
  (`SceneComponent.K2_AttachToComponent` (`self.Gun`) (`self.Mesh`) "WeaponSocket" "SnapToTarget" "SnapToTarget" "SnapToTarget" true)
  (bind _asweapon (cast `/Game/Assets/Guns/Weapon` (`ChildActorComponent.ChildActor` (`self.Gun`))))
  (set `self.CurrentGun` _asweapon))