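; Base enemy weapon Blueprint that sets itself up as "EnemyRifle" on BeginPlay and fires projectiles at the player.
; CalculateDirection traces against static world geometry from a muzzle-derived start toward player 0, aiming from the muzzle socket at the blocking impact or the player's location.
; SpawnProjectile plays the rifle shoot montage, passes that aim through CalculateFinalDirection, and spawns Enemy_Proj with the resulting transform.
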(event `self.ReceiveBeginPlay`
  (`self.Construct` "EnemyRifle")
  (`parent.ReceiveBeginPlay`))

(fn `CalculateDirection`
  (returns (Location :type "Vector Structure") (Rotation :type "Rotator Structure"))
  (bind _returnvalue (`self.MuzzlePozition`))
  (bind _returnvalue_2 (`self.K2_GetActorLocation` (`GameplayStatics.GetPlayerCharacter` 0)))
  (bind _returnvalue_location (`KismetMathLibrary.BreakTransform` (`SceneComponent.K2_GetComponentToWorld` (`self.Muzzle`))))
  (bind (_outhit _returnvalue_3) (`KismetSystemLibrary.LineTraceSingleForObjects` (+ (* (`KismetMathLibrary.GetForwardVector` (struct)) (`KismetMathLibrary.VSize` (- _returnvalue_location (`self.MuzzlePozition`)))) _returnvalue_location) _returnvalue_2 (`|MakeArray` "ObjectTypeQuery1" :!type "EObjectTypeQuery Enum")))
  (return _returnvalue (`KismetMathLibrary.FindLookAtRotation` _returnvalue (`KismetMathLibrary.SelectVector` (`.ImpactPoint` (`GameplayStatics.BreakHitResult` _outhit)) _returnvalue_2 _returnvalue_3))))

(fn `SpawnProjectile`
  (`AnimInstance.Montage_Play` (`SkeletalMeshComponent.GetAnimInstance` (`self.Weapon_Mesh`)) "/Game/Anims/Weapon/Rifle_Shoot_Montage.Rifle_Shoot_Montage" 1.0 "Duration" 0.0 true)
  (bind (_location _rotation) (`self.CalculateDirection`))
  (bind _transform (`self.CalculateFinalDirection` _location _rotation))
  (`|SpawnActorFromClass` "/Game/Assets/Guns/Enemy_Proj.Enemy_Proj_C" _transform "Undefined" "OverrideRootScale" null null))

(fn `UserConstructionScript`
  (`parent.UserConstructionScript`))